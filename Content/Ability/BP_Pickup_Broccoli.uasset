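; Broccoli pickup actor that changes between a Real World and an Imagine World state and disappears when the player hits it.
; In the Imagine World it takes a see-through material and turns off mesh and actor collision; in the Real World it restores its solid material and collision.
; A mesh hit from PlayerCharacter destroys the actor, with no other effect applied here.
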(event `self.ReceiveBeginPlay`
  (`parent.ReceiveBeginPlay`))

(event `self.ToggleToImagineWorld`
  (bind _staticmesh (`self.StaticMesh`))
  (`PrimitiveComponent.SetMaterial` _staticmesh 0 "/Game/Assets/Materials/VegeColours/SeethroghBroccoli_Mat_Inst.SeethroghBroccoli_Mat_Inst")
  (`PrimitiveComponent.SetCollisionEnabled` _staticmesh "NoCollision")
  (`self.SetActorEnableCollision` false))

(event `self.ToggleToRealWorld`
  (bind _staticmesh (`self.StaticMesh`))
  (`PrimitiveComponent.SetMaterial` _staticmesh 0 "/Game/Assets/Props/Veges/lambert2.lambert2")
  (`PrimitiveComponent.SetCollisionEnabled` _staticmesh "QueryAndPhysics")
  (`self.SetActorEnableCollision` true))

(event `self.StaticMesh.OnComponentHit`
  (params (HitComponent :type "PrimitiveComponent Object Reference") (OtherActor :type "Actor Object Reference") (OtherComp :type "PrimitiveComponent Object Reference") (NormalImpulse :type "Vector Structure") (Hit :type "HitResult Structure (by ref)"))
  (cast `PlayerCharacter` OtherActor)
  (`self.K2_DestroyActor`))

(fn `UserConstructionScript`
  (`parent.UserConstructionScript`))