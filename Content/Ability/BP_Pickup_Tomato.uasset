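; Tomato pickup actor that changes state between the game's real and imagine worlds and disappears when the player hits it.
; The imagine-world event swaps the mesh to a see-through material and disables actor collision.
; The real-world event restores the tomato material and collision.
; A mesh hit from PlayerCharacter destroys the actor, with no other pickup effect applied here.
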(event `self.ToggleToImagineWorld`
  (`PrimitiveComponent.SetMaterial` (`self.StaticMesh`) 0 "/Game/Assets/Materials/VegeColours/SeethroghTomato_Mat_Inst.SeethroghTomato_Mat_Inst")
  (`self.SetActorEnableCollision` false))

(event `self.ToggleToRealWorld`
  (`PrimitiveComponent.SetMaterial` (`self.StaticMesh`) 0 "/Game/Assets/Props/Veges/Tomato1.Tomato1")
  (`self.SetActorEnableCollision` true))

(event `self.StaticMesh.OnComponentHit`
  (params (HitComponent :type "PrimitiveComponent Object Reference") (OtherActor :type "Actor Object Reference") (OtherComp :type "PrimitiveComponent Object Reference") (NormalImpulse :type "Vector Structure") (Hit :type "HitResult Structure (by ref)"))
  (cast `PlayerCharacter` OtherActor)
  (`self.K2_DestroyActor`))

(fn `UserConstructionScript`
  (`parent.UserConstructionScript`))