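; Mushroom pickup actor that exists across the game's real and imagine worlds and is removed when the player touches it.
; BeginPlay spawns an item-spawn particle effect at its location and stores the reference.
; World-toggle events swap the mesh material and collision, making it see-through and non-collidable in the imagine world, solid in the real one.
; A mesh hit by PlayerCharacter destroys the mesh and actor, granting nothing here.
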(event `self.ReceiveBeginPlay`
  (`parent.ReceiveBeginPlay`)
  (bind _returnvalue (`GameplayStatics.SpawnEmitterAtLocation` "/Game/VFX/ItemSpawn/ItemSpawn_VFX.ItemSpawn_VFX" (`self.K2_GetActorLocation`)))
  (set `self.ItemSpawn` _returnvalue))

(event `self.ToggleToImagineWorld`
  (bind _staticmesh (`self.StaticMesh`))
  (`PrimitiveComponent.SetMaterial` _staticmesh 0 "/Game/Assets/Materials/VegeColours/SeethroghMushroom_Mat_Inst.SeethroghMushroom_Mat_Inst")
  (`PrimitiveComponent.SetCollisionEnabled` _staticmesh "NoCollision")
  (`self.SetActorEnableCollision` false))

(event `self.ToggleToRealWorld`
  (bind _staticmesh (`self.StaticMesh`))
  (`PrimitiveComponent.SetMaterial` _staticmesh 0 "/Game/Assets/Props/Veges/lambert3.lambert3")
  (`PrimitiveComponent.SetCollisionEnabled` _staticmesh "QueryAndPhysics")
  (`self.SetActorEnableCollision` true))

(event `self.StaticMesh.OnComponentHit`
  (params (HitComponent :type "PrimitiveComponent Object Reference") (OtherActor :type "Actor Object Reference") (OtherComp :type "PrimitiveComponent Object Reference") (NormalImpulse :type "Vector Structure") (Hit :type "HitResult Structure (by ref)"))
  (cast `PlayerCharacter` OtherActor)
  (`ActorComponent.K2_DestroyComponent` (`self.StaticMesh`))
  (`self.K2_DestroyActor`))

(fn `UserConstructionScript`
  (`parent.UserConstructionScript`))