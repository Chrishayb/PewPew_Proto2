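; BP_Bin is a real-world bin where the player deposits collected tomatoes, broccoli or mushrooms to shut down its linked enemy spawner.
; Game mode world toggles show either the bin or the spawner, hiding the other.
; Inside the box, holding E or F moves one item matching EnemyType per tick, updating the counter text.
; Once full, Tick disables the spawner and repeatedly calls the game mode's CheckBinDischarge.
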(event `self.ReceiveBeginPlay`
  ;[1 1 1] BeginPlay
  (bind _asbp_player_character (cast `/Game/Blueprints/BP_PlayerCharacter` (`GameplayStatics.GetPlayerCharacter` 0)))
  (set `self.PlayerRef` _asbp_player_character)
  (bind _asbp_portal_defense_gamemode (cast `/Game/Blueprints/Gamemodes/BP_PortalDefenseGamemode` (`GameplayStatics.GetGameMode`)))
  (add `PortalDefenseGameMode.OnToggleToRealWorld` _asbp_portal_defense_gamemode (delegate `ToggleToRealWorld`))
  (add `PortalDefenseGameMode.OnToggleToImagineWorld` _asbp_portal_defense_gamemode (delegate `ToggleToImagineWorld`))
  (set `self.MaxItem` (`self.NumberOfItemToDischarge`))
  (`TextRenderComponent.K2_SetText` (`TextRenderActor.TextRender` (`self.Text`)) (`KismetTextLibrary.Conv_StringToText` (`KismetStringLibrary.Concat_StrStr` (`KismetStringLibrary.Concat_StrStr` (`KismetStringLibrary.Conv_IntToString` (`self.CurrentItemIn`)) "/") (`KismetStringLibrary.Conv_IntToString` (`self.MaxItem`)))))
  (if (`PortalDefenseGameMode.bInRealWorld` _asbp_portal_defense_gamemode)
    (`self.ToggleToRealWorld`)
    (else
      (`self.ToggleToImagineWorld`))))

(event `ToggleToRealWorld`
  ;[1 1 1] BeginPlay
  (`self.SetActorHiddenInGame` false)
  (`self.SetActorEnableCollision` true)
  (`self.SetActorHiddenInGame` (`self.LinkedSpawner`) true))

(event `ToggleToImagineWorld`
  ;[1 1 1] BeginPlay
  (`self.SetActorHiddenInGame` true)
  (`self.SetActorEnableCollision` false)
  (`self.SetActorHiddenInGame` (`self.LinkedSpawner`) false))

(event `self.ReceiveTick`
  (params (DeltaSeconds :type "Float (single-precision)"))
  ;[1 1 1] Event Tick
  (if (<= (`self.NumberOfItemToDischarge`) 0)
    (set `/Game/Blueprints/BP_EnemySpawner.bSpawnerEnabled` false (`self.LinkedSpawner`))
    (set `self.bDischarged` true)
    (bind _asbp_portal_defense_gamemode (cast `/Game/Blueprints/Gamemodes/BP_PortalDefenseGamemode` (`GameplayStatics.GetGameMode`)))
    (`/Game/Blueprints/Gamemodes/BP_PortalDefenseGamemode.CheckBinDischarge` _asbp_portal_defense_gamemode)
    (elif (`self.Ispress`)
      (if (== (`self.EnemyType`) 1)
        (if (> (`PlayerCharacter.iTomatoCollected` (`self.PlayerRef`)) 0)
          (`PlayerCharacter.UpTomatoCount` (`self.PlayerRef`) -1)
          (`/Engine/EditorBlueprintResources/StandardMacros.DecrementInt` (`self.NumberOfItemToDischarge`) :!label _label
            (:`  `
              (`/Engine/EditorBlueprintResources/StandardMacros.IncrementInt` (`self.CurrentItemIn`)
                (:`  `
                  (`TextRenderComponent.K2_SetText` (`TextRenderActor.TextRender` (`self.Text`)) (`KismetTextLibrary.Conv_StringToText` (`KismetStringLibrary.Concat_StrStr` (`KismetStringLibrary.Concat_StrStr` (`KismetStringLibrary.Conv_IntToString` (`self.CurrentItemIn`)) "/") (`KismetStringLibrary.Conv_IntToString` (`self.MaxItem`))))))))))
        (elif (== (`self.EnemyType`) 2)
          (if (> (`PlayerCharacter.iBrocolliCollected` (`self.PlayerRef`)) 0)
            (`PlayerCharacter.UpBroccoliCount` (`self.PlayerRef`) -1)
            (goto _label))
          (elif (== (`self.EnemyType`) 3)
            (if (> (`PlayerCharacter.iMushroomCollected` (`self.PlayerRef`)) 0)
              (`PlayerCharacter.UpMushroomCount` (`self.PlayerRef`) -1)
              (goto _label))))))))

(event `self.box.OnComponentBeginOverlap`
  (params (OverlappedComponent :type "PrimitiveComponent Object Reference") (OtherActor :type "Actor Object Reference") (OtherComp :type "PrimitiveComponent Object Reference") (OtherBodyIndex :type Integer) (bFromSweep :type Boolean) (SweepResult :type "HitResult Structure (by ref)"))
  (cast `PlayerCharacter` OtherActor)
  (`self.EnableInput` (`GameplayStatics.GetPlayerController` 0)))

(event `Key|F`
  (params (Key :type "Key Structure"))
  (:`Pressed`
    (set `self.Ispress` true))
  (:`Released`
    (set `self.Ispress` false)))

(event `Key|E`
  (params (Key :type "Key Structure"))
  (:`Pressed`
    (set `self.Ispress` true))
  (:`Released`
    (set `self.Ispress` false)))

(event `self.box.OnComponentEndOverlap`
  (params (OverlappedComponent :type "PrimitiveComponent Object Reference") (OtherActor :type "Actor Object Reference") (OtherComp :type "PrimitiveComponent Object Reference") (OtherBodyIndex :type Integer))
  (cast `PlayerCharacter` OtherActor)
  (`self.DisableInput` (`GameplayStatics.GetPlayerController` 0))
  (set `self.Ispress` false))

(fn `UserConstructionScript`)