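; Tomato enemy Blueprint that stores health, movement and death behavior for an enemy targeting the player.
; BeginPlay caches the player pawn, default walk speed and material, and SetMoveSpeed overrides walk speed.
; The damage event lowers health and flags a hit, without checking for death itself.
; The death event plays poof VFX and sound (at world origin), occasionally drops an item and destroys the actor; the GameMode death notification is unwired.
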(event `self.ReceiveBeginPlay`
  ;[1 1 1] Begin Play
  (set `self.TargetToFollow` (`GameplayStatics.GetPlayerPawn` 0))
  (set `self.DefaultMoveSpeed` (`CharacterMovementComponent.MaxWalkSpeed` (`self.CharacterMovement`)))
  (set `self.DefaultMaterial` (`self.DefaultMaterial_0`)))

(event `self.ReceiveTick`
  (params (DeltaSeconds :type "Float (single-precision)")))

(event `self.Receive_ReceivePlayerDamage`
  (params (_damage :type "Float (single-precision)"))
  ;[1 1 1] TakeDamage
  (set `self.CurrentHealth` (- (`self.CurrentHealth`) _damage))
  (set `self.IsTakingDamage` true))

(event `self.Receive_OnDeath`
  ;[1 1 1] OnDeath
  (`GameplayStatics.SpawnEmitterAtLocation` "/Game/VFX/Poof/Poof_VFX.Poof_VFX" (`self.K2_GetActorLocation`))
  (`GameplayStatics.PlaySoundAtLocation` "/Game/Sounds/poof.poof" (0.0 0.0 0.0) (struct) 1.0 1.0 0.0 null null null)
  (if (== (`KismetMathLibrary.RandomIntegerInRange` 0 9) 0)
    (`|SpawnActorFromClass` (`self.ItemToDrop`) (`self.GetTransform`) "Undefined" "OverrideRootScale" null null))
  (`self.K2_DestroyActor`))

(fn `SetMoveSpeed`
  (params (NewSpeed :type "Float (double-precision)"))
  (set `CharacterMovementComponent.MaxWalkSpeed` NewSpeed (`self.CharacterMovement`)))

(fn `UserConstructionScript`)