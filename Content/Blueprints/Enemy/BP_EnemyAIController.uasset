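; AI controller for BP_Enemy that drives it with a behavior tree and blackboard.
; On BeginPlay it casts and caches the controlled pawn, stores its starting position as HomeLocation, then runs BP_EnemyBehaviorTree.
; Every tick it copies the enemy's TargetToFollow and CanMove variables into the blackboard, so the pawn owns that state and the controller only mirrors it for the tree.
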(event `self.ReceiveBeginPlay`
  ;[1 1 1] Initialize Blackboard and Behaviour Tree
  (bind _asbp_enemy (cast `/Game/Blueprints/Enemy/BP_Enemy` (`self.K2_GetPawn`)))
  (set `self.Enemy` _asbp_enemy)
  (bind _blackboardcomponent (`self.UseBlackboard` "/Game/Blueprints/Enemy/BP_EnemyBlackboard.BP_EnemyBlackboard"))
  (`BlackboardComponent.SetValueAsVector` _blackboardcomponent (`self.HomeLocation`) (`self.K2_GetActorLocation` (`self.K2_GetPawn`)))
  (`self.UpdateCanMove`)
  (`self.RunBehaviorTree` "/Game/Blueprints/Enemy/BP_EnemyBehaviorTree.BP_EnemyBehaviorTree"))

(event `self.ReceiveTick`
  (params (DeltaSeconds :type "Float (single-precision)"))
  ;[1 1 1] Event Tick
  ;;[1 1 1] Update Blackboard Variables
  (`self.UpdateTargetToFollow`)
  (`self.UpdateCanMove`))

(event `UpdateTargetToFollow`
  ;[1 1 1] Update TargetToFollow
  (`BlackboardComponent.SetValueAsObject` (`AIBlueprintHelperLibrary.GetBlackboard` null) "TargetToFollow" (`/Game/Blueprints/Enemy/BP_Enemy.TargetToFollow` (`self.Enemy`))))

(event `UpdateCanMove`
  ;[1 1 1] Update CanMove Boolean
  (`BlackboardComponent.SetValueAsBool` (`AIBlueprintHelperLibrary.GetBlackboard` null) "CanMove" (`/Game/Blueprints/Enemy/BP_Enemy.CanMove` (`self.Enemy`))))

(fn `UserConstructionScript`)