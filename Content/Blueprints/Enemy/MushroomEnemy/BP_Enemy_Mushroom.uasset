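; Mushroom enemy Blueprint that targets the player pawn, attacks in melee range and tracks damage taken.
; Tick checks distance to the player, toggling CanMove and playing the attack montage once until CanAttack, which acts as an already-attacking flag, is cleared externally.
; BeginPlay hands its anim Blueprint a self reference.
; Death spawns poof VFX, plays a sound at world origin, drops an item one time in ten and destroys the actor.
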(event `self.ReceiveBeginPlay`
  ;[1 1 1] Begin Play
  (set `self.TargetToFollow` (`GameplayStatics.GetPlayerPawn` 0))
  (set `self.DefaultMoveSpeed` (`CharacterMovementComponent.MaxWalkSpeed` (`self.CharacterMovement`)))
  (set `self.DefaultMaterial` (`self.DefaultMaterial_0`))
  (bind _asabp_enemy_mushroom (cast `/Game/Assets/mushroom_enemy/ABP_Enemy_Mushroom` (`SkeletalMeshComponent.GetAnimInstance` (`self.Mesh`))))
  (set `/Game/Assets/mushroom_enemy/ABP_Enemy_Mushroom.EnemyREF` self _asabp_enemy_mushroom))

(event `self.ReceiveTick`
  (params (DeltaSeconds :type "Float (single-precision)"))
  ;[1 1 1] Event Tick
  (bind _inrange (`self.CheckPlayerInRange`))
  (if _inrange
    (set `self.CanMove` false)
    (if (not (`self.CanAttack`))
      (bind _asabp_enemy_mushroom (cast `/Game/Assets/mushroom_enemy/ABP_Enemy_Mushroom` (`SkeletalMeshComponent.GetAnimInstance` (`self.Mesh`))))
      (`AnimInstance.Montage_Play` _asabp_enemy_mushroom "/Game/Assets/mushroom_enemy/anim/mushroom_enemy_attack_Montage.mushroom_enemy_attack_Montage" 1.0 "MontageLength" 0.0 true)
      (set `self.CanAttack` true))
    (else
      (set `self.CanMove` true))))

(event `self.Receive_ReceivePlayerDamage`
  (params (_damage :type "Float (single-precision)"))
  ;[1 1 1] TakeDamage
  (set `self.CurrentHealth` (- (`self.CurrentHealth`) _damage))
  (set `self.IsTakingDamage` true))

(event `self.Receive_OnDeath`
  ;[1 1 1] OnDeath
  (`GameplayStatics.SpawnEmitterAtLocation` "/Game/VFX/Poof/Poof_VFX.Poof_VFX" (`self.K2_GetActorLocation`))
  (`GameplayStatics.PlaySoundAtLocation` "/Game/Sounds/poof.poof" (0.0 0.0 0.0) (struct) 1.0 1.0 0.0 null null null)
  (if (== (`KismetMathLibrary.RandomIntegerInRange` 0 9) 0)
    (`|SpawnActorFromClass` (`self.ItemToDrop`) (`self.GetTransform`) "Undefined" "OverrideRootScale" null null))
  (`self.K2_DestroyActor`))

(fn `CheckPlayerInRange`
  (returns (InRange :type Boolean) (Distance :type "Float (double-precision)"))
  (bind _returnvalue (`self.GetDistanceTo` (`self.TargetToFollow`)))
  (return (<= _returnvalue (`self.AttackRange`)) _returnvalue))

(fn `SetMoveSpeed`
  (params (NewSpeed :type "Float (double-precision)"))
  (set `CharacterMovementComponent.MaxWalkSpeed` NewSpeed (`self.CharacterMovement`)))

(fn `UserConstructionScript`)