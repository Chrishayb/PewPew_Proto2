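; Boss enemy that tracks the first player, stops to play a smash montage within attack range, and swaps walk speed between real and imaginary worlds.
; Tick sets movement and attack flags, while its animation blueprint receives a self reference, plays the montage and turns red on damage.
; Death spawns poof effects and a random item drop, destroys the actor, shows the next-wave widget, then calls a level load after a delay.
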(event `self.ReceiveBeginPlay`
  ;[1 1 1] Begin Play
  (set `self.TargetToFollow` (`GameplayStatics.GetPlayerPawn` 0))
  (set `self.DefaultMoveSpeed` (`CharacterMovementComponent.MaxWalkSpeed` (`self.CharacterMovement`)))
  (set `self.DefaultMaterial` (`self.DefaultMaterial_0`))
  (bind _asabp_enemy_boss (cast `/Game/Assets/boss/ABP_Enemy_Boss` (`SkeletalMeshComponent.GetAnimInstance` (`self.Mesh`))))
  (set `/Game/Assets/boss/ABP_Enemy_Boss.EnemyREF` self _asabp_enemy_boss)
  (`self.SetWorldMoveSpeeds` (`CharacterMovementComponent.MaxWalkSpeed` (`self.CharacterMovement`))))

(event `self.ReceiveTick`
  (params (DeltaSeconds :type "Float (single-precision)"))
  ;[1 1 1] Event Tick
  (bind _inrange (`self.CheckPlayerInRange`))
  (if _inrange
    (set `self.CanMove` false)
    (if (not (and (`self.CanAttack`) (`self.AbleToAttack`)))
      (bind _asabp_enemy_boss (cast `/Game/Assets/boss/ABP_Enemy_Boss` (`SkeletalMeshComponent.GetAnimInstance` (`self.Mesh`))))
      (`AnimInstance.Montage_Play` _asabp_enemy_boss "/Game/Assets/boss/anim/boss_hulk_smash_Montage.boss_hulk_smash_Montage" 1.0 "MontageLength" 0.0 true)
      (set `self.CanAttack` true))
    (else
      (set `self.CanMove` true))))

(event `self.Receive_ReceivePlayerDamage`
  (params (_damage :type "Float (single-precision)"))
  ;[1 1 1] TakeDamage
  (set `self.CurrentHealth` (- (`self.CurrentHealth`) _damage))
  (set `self.IsTakingDamage` true)
  (bind _asabp_enemy_boss (cast `/Game/Assets/boss/ABP_Enemy_Boss` (`SkeletalMeshComponent.GetAnimInstance` (`self.Mesh`))))
  (`/Game/Assets/boss/ABP_Enemy_Boss.AnimNotify_TurnRed` _asabp_enemy_boss))

(event `self.Receive_OnDeath`
  (bind _returnvalue (`self.K2_GetActorLocation`))
  ;[1 1 1] OnDeath
  (`GameplayStatics.SpawnEmitterAtLocation` "/Game/VFX/Poof/Poof_VFX.Poof_VFX" _returnvalue)
  (`GameplayStatics.PlaySoundAtLocation` "/Game/Sounds/poof.poof" _returnvalue (struct) 1.0 1.0 0.0 null null null)
  (if (== (`KismetMathLibrary.RandomIntegerInRange` 0 9) 0)
    (`|SpawnActorFromClass` (`self.ItemToDrop`) (`self.GetTransform`) "Undefined" "OverrideRootScale" null null))
  (`self.K2_DestroyActor`)
  (bind _returnvalue_2 (`|CreateWidget` "/Game/Assets/UI/Next_Wave.Next_Wave_C" (`GameplayStatics.GetPlayerController` 0)))
  (`UserWidget.AddToViewport` _returnvalue_2 0)
  (`KismetSystemLibrary.Delay` 5.0)
  (`GameplayStatics.OpenLevel` "GAMEPLAY_YIKES_2"))

(event `self.Receive_SwapToImagineWorld`
  ;[1 1 1] Change To Imaginary Move Speed
  (set `CharacterMovementComponent.MaxWalkSpeed` (`self.ImaginaryMoveSpeed`) (`self.CharacterMovement`)))

(event `self.Receive_SwapToRealWorld`
  ;[1 1 1] Change To Real Move Speed
  (set `CharacterMovementComponent.MaxWalkSpeed` (`self.RealMoveSpeed`) (`self.CharacterMovement`)))

(fn `CheckPlayerInRange`
  (returns (InRange :type Boolean) (Distance :type "Float (double-precision)"))
  (bind _returnvalue (`self.GetDistanceTo` (`self.TargetToFollow`)))
  (return (<= _returnvalue (`self.AttackRange`)) _returnvalue))

(fn `SetMoveSpeed`
  (params (NewSpeed :type "Float (double-precision)"))
  (set `CharacterMovementComponent.MaxWalkSpeed` NewSpeed (`self.CharacterMovement`)))

(fn `UserConstructionScript`)