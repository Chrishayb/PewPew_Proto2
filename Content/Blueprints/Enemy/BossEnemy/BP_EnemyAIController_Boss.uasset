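; AI controller for the boss enemy that drives it through the boss behavior tree and blackboard.
; BeginPlay sets up the blackboard, while possession records the pawn's location as HomeLocation and starts the tree.
; Every Tick it casts the pawn to BP_Enemy_Boss and copies its TargetToFollow and CanMove into the blackboard, so the tree follows the pawn's state by polling.
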(event `self.ReceiveBeginPlay`
  ;[1 1 1] Initialize Blackboard and Behaviour Tree
  (`self.UseBlackboard` "/Game/Blueprints/Enemy/BossEnemy/BP_EnemyBlackboard_Boss.BP_EnemyBlackboard_Boss"))

(event `self.OnPossess`
  (params (PossessedPawn :type "Pawn Object Reference"))
  (bind _returnvalue (`AIBlueprintHelperLibrary.GetBlackboard` null))
  ;[1 1 1] OnPossess
  (set `self.Enemy` (`self.Enemy`))
  (`/Engine/EditorBlueprintResources/StandardMacros.IsValid` _returnvalue
    (:`Is Valid`
      (`BlackboardComponent.SetValueAsVector` _returnvalue (`self.HomeLocation`) (`self.K2_GetActorLocation` (`self.K2_GetPawn`))))
    (:`Is Not Valid`
      _))
  (`self.UpdateCanMove`)
  (`self.RunBehaviorTree` "/Game/Blueprints/Enemy/BossEnemy/BP_BossEnemyBehaviorTree.BP_BossEnemyBehaviorTree"))

(event `self.ReceiveTick`
  (params (DeltaSeconds :type "Float (single-precision)"))
  (bind _asbp_enemy_boss (cast `/Game/Blueprints/Enemy/BossEnemy/BP_Enemy_Boss` (`self.K2_GetPawn`)))
  (`/Engine/EditorBlueprintResources/StandardMacros.IsValid` _asbp_enemy_boss
    (:`Is Valid`
      (set `self.Enemy` _asbp_enemy_boss)
      ;[1 1 1] Event Tick
      ;;[1 1 1] Update Blackboard Variables
      (`self.UpdateTargetToFollow`)
      (`self.UpdateCanMove`))))

(event `UpdateTargetToFollow`
  (bind _returnvalue (`AIBlueprintHelperLibrary.GetBlackboard` null))
  ;[1 1 1] Update TargetToFollow
  (`/Engine/EditorBlueprintResources/StandardMacros.IsValid` _returnvalue
    (:`Is Valid`
      (`BlackboardComponent.SetValueAsObject` _returnvalue "TargetToFollow" (`/Game/Blueprints/Enemy/BossEnemy/BP_Enemy_Boss.TargetToFollow` (`self.Enemy`))))))

(event `UpdateCanMove`
  (bind _returnvalue (`AIBlueprintHelperLibrary.GetBlackboard` null))
  ;[1 1 1] Update CanMove Boolean
  (`/Engine/EditorBlueprintResources/StandardMacros.IsValid` _returnvalue
    (:`Is Valid`
      (`BlackboardComponent.SetValueAsBool` _returnvalue "CanMove" (`EnemyBase.CanMove` (`self.Enemy`))))))

(fn `UserConstructionScript`)