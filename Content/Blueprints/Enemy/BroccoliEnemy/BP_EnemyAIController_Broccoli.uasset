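; AI controller for the Broccoli enemy that drives it with a Blackboard and Behavior Tree.
; On BeginPlay it caches the controlled pawn, sets up the Blackboard with the spawn position as HomeLocation, then runs the Broccoli behavior tree.
; Every Tick it copies the pawn's TargetToFollow and CanMove into the Blackboard, so the tree reads state owned by the enemy.
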(event `self.ReceiveBeginPlay`
  ;[1 1 1] Initialize Blackboard and Behaviour Tree
  (bind _asbp_enemy_broccoli (cast `/Game/Blueprints/Enemy/BroccoliEnemy/BP_Enemy_Broccoli` (`self.K2_GetPawn`)))
  (set `self.Enemy` _asbp_enemy_broccoli)
  (bind _blackboardcomponent (`self.UseBlackboard` "/Game/Blueprints/Enemy/BroccoliEnemy/BP_EnemyBlackboard_Broccoli.BP_EnemyBlackboard_Broccoli"))
  (`BlackboardComponent.SetValueAsVector` _blackboardcomponent (`self.HomeLocation`) (`self.K2_GetActorLocation` (`self.K2_GetPawn`)))
  (`self.UpdateCanMove`)
  (`self.RunBehaviorTree` "/Game/Blueprints/Enemy/BroccoliEnemy/BP_BroccoliEnemyBehaviorTree.BP_BroccoliEnemyBehaviorTree"))

(event `self.ReceiveTick`
  (params (DeltaSeconds :type "Float (single-precision)"))
  ;[1 1 1] Event Tick
  ;;[1 1 1] Update Blackboard Variables
  (`self.UpdateTargetToFollow`)
  (`self.UpdateCanMove`))

(event `UpdateTargetToFollow`
  ;[1 1 1] Update TargetToFollow
  (`BlackboardComponent.SetValueAsObject` (`AIBlueprintHelperLibrary.GetBlackboard` null) "TargetToFollow" (`/Game/Blueprints/Enemy/BroccoliEnemy/BP_Enemy_Broccoli.TargetToFollow` (`self.Enemy`))))

(event `UpdateCanMove`
  ;[1 1 1] Update CanMove Boolean
  (`BlackboardComponent.SetValueAsBool` (`AIBlueprintHelperLibrary.GetBlackboard` null) "CanMove" (`/Game/Blueprints/Enemy/BroccoliEnemy/BP_Enemy_Broccoli.CanMove` (`self.Enemy`))))

(fn `UserConstructionScript`)