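; Broccoli enemy character Blueprint that tracks its health and movement speed.
; On BeginPlay it stores the player pawn as its follow target and caches the default walk speed.
; A player-damage event subtracts from current health, with no death check here, and SetMoveSpeed overrides the max walk speed.
; The graphs shown contain no follow logic, and Tick is empty.
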(event `self.ReceiveBeginPlay`
  ;[1 1 1] Begin Play
  (set `self.TargetToFollow` (`GameplayStatics.GetPlayerPawn` 0))
  (set `self.DefaultMoveSpeed` (`CharacterMovementComponent.MaxWalkSpeed` (`self.CharacterMovement`))))

(event `self.ReceiveTick`
  (params (DeltaSeconds :type "Float (single-precision)")))

(event `self.Receive_ReceivePlayerDamage`
  (params (_damage :type "Float (single-precision)"))
  ;[1 1 1] TakeDamage
  (set `self.CurrentHealth` (- (`self.CurrentHealth`) _damage)))

(fn `SetMoveSpeed`
  (params (NewSpeed :type "Float (double-precision)"))
  (set `CharacterMovementComponent.MaxWalkSpeed` NewSpeed (`self.CharacterMovement`)))

(fn `UserConstructionScript`)