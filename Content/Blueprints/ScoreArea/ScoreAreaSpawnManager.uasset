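; ScoreAreaSpawnManager keeps score areas spawned at preset locations, up to a MaxSpawnArea limit.
; Each tick while the BP_PewPewTestGamemode ScoreAreaCount is below that limit, it picks a random ScoreAreaSpawnLocation entry.
; If that entry has no valid ScoreAreaRef, it spawns a ScoreArea at its transform and increments the count.
; The random range includes the array length, so picks can fall out of bounds.
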(event `self.ReceiveBeginPlay`
  (bind _asbp_pew_pew_test_gamemode (cast `/Game/Blueprints/BP_PewPewTestGamemode` (`GameplayStatics.GetGameMode`))))

(event `self.ReceiveTick`
  (params (DeltaSeconds :type "Float (single-precision)"))
  (bind _scoreareaspawnlocation (`self.ScoreAreaSpawnLocation`))
  (bind _scoreareacount (`/Game/Blueprints/BP_PewPewTestGamemode.ScoreAreaCount` (stale `self.ReceiveBeginPlay` _asbp_pew_pew_test_gamemode)))
  (if (< _scoreareacount (`self.MaxSpawnArea`))
    (bind _output_get (set `self.Random Value` (`KismetMathLibrary.RandomIntegerInRange` 0 (`KismetArrayLibrary.Array_Length` _scoreareaspawnlocation))))
    (bind _output (`|GetArrayItem` _scoreareaspawnlocation _output_get))
    (`/Engine/EditorBlueprintResources/StandardMacros.IsValid` (`/Game/Blueprints/ScoreArea/ScoreAreaSpawnLocation.ScoreAreaRef` _output)
      (:`Is Not Valid`
        (`|SpawnActorFromClass` (`self.ScoreArea`) (`self.GetTransform` _output) "Undefined" "OverrideRootScale" null null)
        (`/Engine/EditorBlueprintResources/StandardMacros.IncrementInt` _scoreareacount)))))

(fn `UserConstructionScript`)