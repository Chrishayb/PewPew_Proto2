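; ScoreArea is an area actor that absorbs enemies entering its sphere and turns into a Boss spawn.
; Each absorbed enemy plays a poof effect and lowers MaxMonsterCount; a player overlap instead calls ToggleWorld on the PortalDefense game mode.
; Tick spawns the Boss and destroys the area when the count runs out, or when AllPotalDisable is set after any count loss.
; With an untouched count, that flag just destroys it.
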(event `self.ReceiveBeginPlay`
  (set `self.DefaultMaxMonsterCount` (`self.MaxMonsterCount`)))

(event `self.ReceiveTick`
  (params (DeltaSeconds :type "Float (single-precision)"))
  (bind (_returnvalue_x _returnvalue_y) (`KismetMathLibrary.BreakVector` (`self.K2_GetActorLocation`)))
  (if (`self.AllPotalDisable`)
    (if (== (`self.MaxMonsterCount`) (`self.DefaultMaxMonsterCount`))
      (`self.K2_DestroyActor`)
      (else
        (`|SpawnActorFromClass` (`self.Boss`) (`self.GetTransform`) "Undefined" "OverrideRootScale" null null)
        (`self.K2_DestroyActor`)))
    (elif (< (`self.MaxMonsterCount`) 1)
      (`self.SetActorEnableCollision` false)
      (`|SpawnActorFromClass` (`self.Boss`) (`KismetMathLibrary.MakeTransform` (`KismetMathLibrary.MakeVector` _returnvalue_x _returnvalue_y 1000.0)) "AdjustIfPossibleButAlwaysSpawn" "OverrideRootScale" null null)
      (`self.K2_DestroyActor`))))

(event `self.Sphere.OnComponentBeginOverlap`
  (params (OverlappedComponent :type "PrimitiveComponent Object Reference") (OtherActor :type "Actor Object Reference") (OtherComp :type "PrimitiveComponent Object Reference") (OtherBodyIndex :type Integer) (bFromSweep :type Boolean) (SweepResult :type "HitResult Structure (by ref)"))
  (bind _asenemy_base (cast `EnemyBase` OtherActor)
    (:`then`
      (`/Engine/EditorBlueprintResources/StandardMacros.DecrementInt` (`self.MaxMonsterCount`)
        (:`  `
          (`GameplayStatics.SpawnEmitterAtLocation` "/Game/VFX/Poof/Poof_VFX.Poof_VFX" (`self.K2_GetActorLocation` _asenemy_base))
          (`self.K2_DestroyActor` _asenemy_base))))
    (:`CastFailed`
      (cast `/Game/Blueprints/BP_PlayerCharacter` OtherActor)
      (bind _asportal_defense_game_mode (cast `PortalDefenseGameMode` (`GameplayStatics.GetGameMode`)))
      (`PortalDefenseGameMode.ToggleWorld` _asportal_defense_game_mode))))

(fn `SpawnBoss`
  (`|SpawnActorFromClass` (`self.Boss`) (`SceneComponent.K2_GetComponentToWorld` (`self.BoosSpawnLocation`)) "Undefined" "OverrideRootScale" null null))

(fn `UserConstructionScript`)