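; EnemySpawnManager periodically spawns random enemy types at random spawn locations.
; BeginPlay starts a looping timer at SpawnRate, which checks the BP_PewPewTestGamemode EnemyArray count against MaxEnemyCount before spawning.
; If the game mode cast fails, it spawns without that cap.
; ChooseRandomSpawnLocation stores a random index, then TrySpawn spawns a random EnemyTypes class at that location's transform.
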(event `self.ReceiveBeginPlay`
  ;[1 1 1] Timer loop on BeginPlay
  (`KismetSystemLibrary.K2_SetTimerDelegate` (delegate `SpawnEnemy`) (`self.SpawnRate`) true))

(event `SpawnEnemy`
  ;[1 1 1] Spawn Enemy
  (bind _asbp_pew_pew_test_gamemode (cast `/Game/Blueprints/Gamemodes/BP_PewPewTestGamemode` (`GameplayStatics.GetGameMode`))
    (:`then`
      (if (< (`KismetArrayLibrary.Array_Length` (`/Game/Blueprints/Gamemodes/BP_PewPewTestGamemode.EnemyArray` _asbp_pew_pew_test_gamemode)) (`self.MaxEnemyCount`))
        (`self.ChooseRandomSpawnLocation` :!label _label)
        (`self.TrySpawn`)))
    (:`CastFailed`
      (goto _label))))

(event `ChooseRandomSpawnLocation`
  ;[1 1 1] Choose Random Spawn Location
  (set `self.RandomInt` (`KismetMathLibrary.RandomIntegerInRange` 0 (- (`KismetArrayLibrary.Array_Length` (`self.SpawnLocations`)) 1))))

(fn `TrySpawn`
  (bind _enemytypes (`self.EnemyTypes`))
  (`|SpawnActorFromClass` (`|GetArrayItem` _enemytypes (`KismetMathLibrary.RandomIntegerInRange` 0 (- (`KismetArrayLibrary.Array_Length` _enemytypes) 1))) (`self.GetTransform` (`|GetArrayItem` (`self.SpawnLocations`) (`self.RandomInt`))) "Undefined" "OverrideRootScale" null null))

(fn `UserConstructionScript`)