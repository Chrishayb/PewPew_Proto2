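; Portal defense game mode that runs phase logic for an adds phase and a boss phase.
; The adds phase enables every enemy spawner; the boss phase disables them and tells the portal, found at BeginPlay and cast to ScoreArea, to spawn the boss.
; CheckBinDischarge switches to the boss phase once no bin remains undischarged.
; Waiting-to-start and end state handlers are empty.
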(event `self.ReceiveBeginPlay`
  (`parent.ReceiveBeginPlay`)
  (bind _outactors (`GameplayStatics.GetAllActorsOfClass` (`self.PortalClass`)))
  (set `self.Portal` (`|GetArrayItem` _outactors)))

(event `self.Receive_HandleWaitingToStartState`)

(event `self.Receive_HandleAddsPhaseState`
  (for _array_element (`self.EnemySpawners`)
    (bind _asbp_enemy_spawner (cast `/Game/Blueprints/BP_EnemySpawner` _array_element))
    (set `/Game/Blueprints/BP_EnemySpawner.bSpawnerEnabled` true _asbp_enemy_spawner)))

(event `self.Receive_HandleBossPhaseState`
  (`self.DisableAllSpawner`)
  (bind _asscore_area (cast `/Game/Blueprints/ScoreArea/ScoreArea` (`self.Portal`)))
  (`/Game/Blueprints/ScoreArea/ScoreArea.SpawnBoss` _asscore_area))

(event `self.Receive_HandleEndState`)

(fn `CheckBinDischarge`
  (for _array_element (`self.Bins`)
    (bind _asbp_bin (cast `/Game/Blueprints/BP_Bin` _array_element)
      (:`then`
        (if (not (`/Game/Blueprints/BP_Bin.bDischarged` _asbp_bin))
          (return)))
      (:`CastFailed`
        (`KismetSystemLibrary.PrintString` "This is not the bin type!"))))
  (`self.SetPortalDefenseState` "BossPhase"))

(fn `DisableAllSpawner`
  (for _array_element (`self.EnemySpawners`)
    (bind _asbp_enemy_spawner (cast `/Game/Blueprints/BP_EnemySpawner` _array_element))
    (set `/Game/Blueprints/BP_EnemySpawner.bSpawnerEnabled` false _asbp_enemy_spawner)))

(fn `UserConstructionScript`)