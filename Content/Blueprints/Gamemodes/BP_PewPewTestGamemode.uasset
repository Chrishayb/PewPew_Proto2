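; Test game mode that switches the game between a "real" world and an "image" world and opens the Darren level when the player dies.
; CurrentWorld flips a flag to run either toggle, changing skybox visibility, the Imageworld enabled state, and fountain and item visibility and collision.
; Real world shows fountains and items and makes enemies see-through with damage disabled; image world reverses this.
; EnemyDeath removes enemies from the tracked array and destroys them.
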(event `self.ReceiveBeginPlay`
  (bind _asbp_player_character (cast `/Game/Blueprints/BP_PlayerCharacter` (`GameplayStatics.GetPlayerCharacter` 0)))
  (add `PlayerCharacter.PlayerDeath` _asbp_player_character (delegate `OnPlayerDeath`))
  (bind _outactors (`GameplayStatics.GetAllActorsOfClass` "/Game/Assets/Materials/Skybok/Skybok_BP.Skybok_BP_C"))
  (set `self.Skybok` (`|GetArrayItem` _outactors)))

(event `OnPlayerDeath`
  (`GameplayStatics.OpenLevel` "Darren"))

(fn `CurrentWorld`
  (bind _output_get (set `self.ToggleWorld` (not (`self.ToggleWorld`))))
  (if _output_get
    (`self.RealWorldToggle`)
    (else
      (`self.ImageWorldToggle`))))

(fn `EnemyDeath`
  (params (EnemyReference :type "EnemyBase Object Reference"))
  (bind _returnvalue (`KismetArrayLibrary.Array_RemoveItem` (`self.EnemyArray`) EnemyReference))
  (if (not _returnvalue)
    (`KismetSystemLibrary.PrintString` "This enemy is not in the array lolz"))
  (`self.K2_DestroyActor` EnemyReference))

(fn `ImageWorldToggle`
  (set `PostProcessComponent.bEnabled` true (`self.imageworld`))
  (`SceneComponent.SetVisibility` (`/Game/Assets/Materials/Skybok/Skybok_BP.StaticMesh` (`self.Skybok`)) true false)
  (for _array_element (`self.WaterFountain`)
    (`SceneComponent.SetVisibility` (`Actor.RootComponent` _array_element) false true)
    (`self.SetActorEnableCollision` _array_element false))
  (for _array_element_2 (`self.ItemArray`)
    (`SceneComponent.SetVisibility` (`Actor.RootComponent` _array_element_2) false true)
    (`self.SetActorEnableCollision` _array_element_2 false))
  (for _array_element_3 (`self.EnemyArray`)
    (`/Engine/EditorBlueprintResources/StandardMacros.IsValid` _array_element_3
      (:`Is Valid`
        (`PrimitiveComponent.SetMaterial` (`Character.Mesh` _array_element_3) 0 (`EnemyBase.DefaultMaterial` _array_element_3))
        (set `EnemyBase.CanDamage` true _array_element_3)))))

(fn `RealWorldToggle`
  (`SceneComponent.SetVisibility` (`/Game/Assets/Materials/Skybok/Skybok_BP.StaticMesh` (`self.Skybok`)) false false)
  (set `PostProcessComponent.bEnabled` false (`self.imageworld`))
  (for _array_element (`self.WaterFountain`)
    (`/Engine/EditorBlueprintResources/StandardMacros.IsValid` _array_element
      (:`Is Valid`
        (`SceneComponent.SetVisibility` (`Actor.RootComponent` _array_element) true true)
        (`self.SetActorEnableCollision` _array_element true))))
  (for _array_element_2 (`self.ItemArray`)
    (`/Engine/EditorBlueprintResources/StandardMacros.IsValid` _array_element_2
      (:`Is Valid`
        (`SceneComponent.SetVisibility` (`/Game/Ability/Item.DefaultSceneRoot` _array_element_2) true true)
        (`self.SetActorEnableCollision` _array_element_2 true))))
  (for _array_element_3 (`self.EnemyArray`)
    (`/Engine/EditorBlueprintResources/StandardMacros.IsValid` _array_element_3
      (:`Is Valid`
        (`PrimitiveComponent.SetMaterial` (`Character.Mesh` _array_element_3) 0 "/Game/Assets/Materials/SeethroughEnemy_Mat.SeethroughEnemy_Mat")
        (set `EnemyBase.CanDamage` false _array_element_3)))))

(fn `UserConstructionScript`)