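; Water fountain actor that hydrates the player while E or F is held inside its trigger box.
; Box overlap enables or disables player input on the fountain; while pressed, Tick shows the VFX and adds hydration every frame, independent of delta time.
; It registers with BP_PewPewTestGamemode, starts hidden if ToggleWorld is false, and extends the parent's world-toggle events to enable collision only in the real world.
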(event `self.ReceiveBeginPlay`
  (`parent.ReceiveBeginPlay`)
  (bind _asbp_pew_pew_test_gamemode (cast `/Game/Blueprints/Gamemodes/BP_PewPewTestGamemode` (`GameplayStatics.GetGameMode`)))
  (`KismetArrayLibrary.Array_Add` (`/Game/Blueprints/Gamemodes/BP_PewPewTestGamemode.WaterFountain` _asbp_pew_pew_test_gamemode) self)
  (if (not (`/Game/Blueprints/Gamemodes/BP_PewPewTestGamemode.ToggleWorld` _asbp_pew_pew_test_gamemode))
    (`SceneComponent.SetVisibility` (`self.RootComponent`) false true)
    (`self.SetActorEnableCollision` false)))

(event `self.ReceiveTick`
  (params (DeltaSeconds :type "Float (single-precision)"))
  (if (`self.Ispress`)
    (`SceneComponent.SetVisibility` (`self.Fountain_VFX`) true true)
    (bind _asplayer_character (cast `PlayerCharacter` (`GameplayStatics.GetPlayerCharacter` 0)))
    (`PlayerCharacter.HydratingByValue` _asplayer_character 1.0)
    (else
      (`SceneComponent.SetVisibility` (`self.Fountain_VFX`) false true))))

(event `self.Box.OnComponentBeginOverlap`
  (params (OverlappedComponent :type "PrimitiveComponent Object Reference") (OtherActor :type "Actor Object Reference") (OtherComp :type "PrimitiveComponent Object Reference") (OtherBodyIndex :type Integer) (bFromSweep :type Boolean) (SweepResult :type "HitResult Structure (by ref)"))
  (cast `PlayerCharacter` OtherActor)
  (`self.EnableInput` (`GameplayStatics.GetPlayerController` 0)))

(event `Key|F`
  (params (Key :type "Key Structure"))
  (:`Pressed`
    (set `self.Ispress` true))
  (:`Released`
    (set `self.Ispress` false)))

(event `Key|E`
  (params (Key :type "Key Structure"))
  (:`Pressed`
    (set `self.Ispress` true))
  (:`Released`
    (set `self.Ispress` false)))

(event `self.Box.OnComponentEndOverlap`
  (params (OverlappedComponent :type "PrimitiveComponent Object Reference") (OtherActor :type "Actor Object Reference") (OtherComp :type "PrimitiveComponent Object Reference") (OtherBodyIndex :type Integer))
  (cast `PlayerCharacter` OtherActor)
  (`self.DisableInput` (`GameplayStatics.GetPlayerController` 0))
  (set `self.Ispress` false))

(event `self.ToggleToImagineWorld`
  (`parent.ToggleToImagineWorld`)
  (`PrimitiveComponent.SetCollisionEnabled` (`self.Collider`) "NoCollision")
  (`PrimitiveComponent.SetCollisionEnabled` (`self.Box`) "NoCollision"))

(event `self.ToggleToRealWorld`
  (`parent.ToggleToRealWorld`)
  (`PrimitiveComponent.SetCollisionEnabled` (`self.Box`) "QueryAndPhysics")
  (`PrimitiveComponent.SetCollisionEnabled` (`self.Collider`) "QueryAndPhysics"))

(fn `UserConstructionScript`)