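; Pinecone pickup that swaps its look between the real world and the imagine world.
; On BeginPlay it binds to the PortalDefenseGameMode world-toggle events, which show one of its two meshes and hide the other.
; When a PlayerCharacter overlaps the real-world mesh, it adds one pinecone to that player and destroys itself.
; The toggle only changes visibility, not collision.
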(event `self.ReceiveBeginPlay`
  (bind _asportal_defense_game_mode (cast `PortalDefenseGameMode` (`GameplayStatics.GetGameMode`))
    (:`then`
      (add `PortalDefenseGameMode.OnToggleToImagineWorld` _asportal_defense_game_mode (delegate `OnToImagineWorld`))
      (add `PortalDefenseGameMode.OnToggleToRealWorld` _asportal_defense_game_mode (delegate `OnToRealWorld`)))
    (:`CastFailed`
      (`KismetSystemLibrary.PrintString` "Its currently not "))))

(event `OnToImagineWorld`
  (`self.ToggleToImagineWorld`))

(event `OnToRealWorld`
  (`self.ToggleToRealWorld`))

(event `self.RealWorldMesh.OnComponentBeginOverlap`
  (params (OverlappedComponent :type "PrimitiveComponent Object Reference") (OtherActor :type "Actor Object Reference") (OtherComp :type "PrimitiveComponent Object Reference") (OtherBodyIndex :type Integer) (bFromSweep :type Boolean) (SweepResult :type "HitResult Structure (by ref)"))
  (bind _asplayer_character (cast `PlayerCharacter` OtherActor))
  (`PlayerCharacter.UpPinecone` _asplayer_character 1)
  (`self.K2_DestroyActor`))

(fn `ToggleToImagineWorld`
  (`SceneComponent.SetVisibility` (`self.RealWorldMesh`) false false)
  (`SceneComponent.SetVisibility` (`self.ImagineWorldMesh`) true false))

(fn `ToggleToRealWorld`
  (`SceneComponent.SetVisibility` (`self.RealWorldMesh`) true false)
  (`SceneComponent.SetVisibility` (`self.ImagineWorldMesh`) false false))

(fn `UserConstructionScript`)