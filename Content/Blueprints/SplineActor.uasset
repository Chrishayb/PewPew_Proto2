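; Spline actor that lays a row of wooden plank meshes along an editable spline, built in the Construction Script.
; It divides the spline length by Spacing and adds a static mesh component at each step, aligned to the spline in local space.
; Small random roll and pitch offsets, plus a rotation flip on every even-indexed plank, break up the repetition.
; The event graph has no active gameplay logic.
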(event `self.ReceiveBeginPlay`)

(fn `UserConstructionScript`
  (bind _splinecomponentexample (`self.SplineComponentExample`))
  (bind _spacing (`self.spacing`))
  (for _index (range (+ (`.ReturnValue` (`KismetMathLibrary.FMod` (`SplineComponent.GetSplineLength` _splinecomponentexample) _spacing)) 1))
    (bind _returnvalue (* _index _spacing))
    (bind (_returnvalue_roll _returnvalue_pitch _returnvalue_yaw) (`KismetMathLibrary.BreakRotator` (`SplineComponent.GetRotationAtDistanceAlongSpline` _splinecomponentexample _returnvalue "Local")))
    (bind _returnvalue_2 (`AddComponent|NODE_AddStaticMeshComponent-0` :`RelativeTransform` (`KismetMathLibrary.MakeTransform` (`SplineComponent.GetLocationAtDistanceAlongSpline` _splinecomponentexample _returnvalue "Local") (`KismetMathLibrary.MakeRotator` (+ _returnvalue_roll (`KismetMathLibrary.RandomFloatInRange` -2.0 2.0)) (+ _returnvalue_pitch (`KismetMathLibrary.RandomFloatInRange` -5.0 5.0)) _returnvalue_yaw))))
    (`StaticMeshComponent.SetStaticMesh` _returnvalue_2 "/Game/Assets/Plank/Plank_low.Plank_low")
    (`PrimitiveComponent.SetMaterial` _returnvalue_2 0 "/Game/Assets/Plank/Plank_low_lambert1_BaseColor_Mat.Plank_low_lambert1_BaseColor_Mat")
    (if (== (mod _index 2) 0)
      (`SceneComponent.K2_AddRelativeRotation` _returnvalue_2 (struct :`Pitch` 180.0 :`Roll` 180.0) false false))))