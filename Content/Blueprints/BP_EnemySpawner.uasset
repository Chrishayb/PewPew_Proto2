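; Enemy spawner that creates enemies at a spawn point and sends each after either the player or the boss portal.
; BeginPlay finds the first ScoreArea as the portal and starts a looping spawn timer, or prints an error if none exists.
; Spawning requires the spawner to be enabled and either per-target array to be below its cap, after pruning invalid enemies.
; Targets are random while both have room, otherwise the one with space.
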(event `self.ReceiveBeginPlay`
  (bind _outactors (`GameplayStatics.GetAllActorsOfClass` "/Game/Blueprints/ScoreArea/ScoreArea.ScoreArea_C"))
  (if (!= (`KismetArrayLibrary.Array_Length` _outactors) 0)
    (set `self.PortalReference` (`|GetArrayItem` _outactors))
    (`KismetSystemLibrary.K2_SetTimerDelegate` (`|CreateDelegate` :!event `SpawnEnemy`) (`self.SpawnDelay`) true)
    (else
      (`KismetSystemLibrary.PrintString` "Error: No boss portal been placed"))))

(fn `GetCanSpawn`
  (returns (Result :type Boolean))
  (`self.VerifyArrays`)
  (return (and (`self.bSpawnerEnabled`) (or (< (`KismetArrayLibrary.Array_Length` (`self.EnemyTargetPortalArray`)) (`self.MaxEnemyTargetPortal`)) (< (`KismetArrayLibrary.Array_Length` (`self.EnemyTargetPlayerArray`)) (`self.MaxEnemyTargetPlayer`))))))

(fn `GetRandomTarget`
  (returns (Target :type "Actor Object Reference"))
  (bind _returnvalue (< (`KismetArrayLibrary.Array_Length` (`self.EnemyTargetPlayerArray`)) (`self.MaxEnemyTargetPlayer`)))
  (if (and (< (`KismetArrayLibrary.Array_Length` (`self.EnemyTargetPortalArray`)) (`self.MaxEnemyTargetPortal`)) _returnvalue)
    (if (`KismetMathLibrary.RandomBool`)
      _
      (else
        (set `self.bTargetingPlayer` false :!label _label)
        (return (`self.PortalReference`))))
    (elif _returnvalue
      _
      (else
        (goto _label))))
  (set `self.bTargetingPlayer` true)
  (return (`GameplayStatics.GetPlayerCharacter` 0)))

(fn `SpawnEnemy`
  (bind _result (`self.GetCanSpawn`))
  (if _result
    (bind _returnvalue (`|SpawnActorFromClass` (`self.EnemyType`) (`SceneComponent.K2_GetComponentToWorld` (`self.SpawnPoint`)) "Undefined" "OverrideRootScale" null null))
    (`/Engine/EditorBlueprintResources/StandardMacros.IsValid` _returnvalue
      (:`Is Valid`
        (bind _target (`self.GetRandomTarget`))
        (if (`self.bTargetingPlayer`)
          (`KismetArrayLibrary.Array_Add` (`self.EnemyTargetPlayerArray`) _returnvalue)
          (else
            (`KismetArrayLibrary.Array_Add` (`self.EnemyTargetPortalArray`) _returnvalue)))
        (`EnemyBase.ChangeTarget` _returnvalue _target)))
    (else
      (`KismetSystemLibrary.PrintString` "I cannot spawn"))))

(fn `UserConstructionScript`)

(fn `VerifyArrays`
  (bind _enemytargetplayerarray (`self.EnemyTargetPlayerArray`))
  (bind _enemytargetportalarray (`self.EnemyTargetPortalArray`))
  (for _array_element _enemytargetplayerarray
    (`/Engine/EditorBlueprintResources/StandardMacros.IsValid` _array_element
      (:`Is Not Valid`
        (`KismetArrayLibrary.Array_RemoveItem` _enemytargetplayerarray _array_element))))
  (for _array_element_2 _enemytargetportalarray
    (`/Engine/EditorBlueprintResources/StandardMacros.IsValid` _array_element_2
      (:`Is Not Valid`
        (`KismetArrayLibrary.Array_RemoveItem` _enemytargetportalarray _array_element_2)))))