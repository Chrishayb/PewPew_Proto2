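; ScoreArea is a capture-zone style actor that awards score while the player is inside its sphere.
; Overlap events from PlayerCharacter toggle an InSphere flag and swap the sphere between green and red dome materials.
; Tick runs through a two-second Delay, acting as a repeating timer that increments CurrentScore on BP_PewPewTestGamemode whenever InSphere is set as the delay completes.
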(event `self.ReceiveTick`
  (params (DeltaSeconds :type "Float (single-precision)"))
  (`KismetSystemLibrary.Delay` 2.0)
  (if (`self.InSphere`)
    (bind _asbp_pew_pew_test_gamemode (cast `/Game/Blueprints/BP_PewPewTestGamemode` (`GameplayStatics.GetGameMode`)))
    (`/Engine/EditorBlueprintResources/StandardMacros.IncrementInt` (`/Game/Blueprints/BP_PewPewTestGamemode.CurrentScore` _asbp_pew_pew_test_gamemode))))

(event `self.Sphere.OnComponentBeginOverlap`
  (params (OverlappedComponent :type "PrimitiveComponent Object Reference") (OtherActor :type "Actor Object Reference") (OtherComp :type "PrimitiveComponent Object Reference") (OtherBodyIndex :type Integer) (bFromSweep :type Boolean) (SweepResult :type "HitResult Structure (by ref)"))
  (cast `PlayerCharacter` OtherActor)
  (`PrimitiveComponent.SetMaterial` (`self.Sphere`) 0 "/Game/Assets/Materials/Dome_Green_Mat_Inst.Dome_Green_Mat_Inst")
  (set `self.InSphere` true))

(event `self.Sphere.OnComponentEndOverlap`
  (params (OverlappedComponent :type "PrimitiveComponent Object Reference") (OtherActor :type "Actor Object Reference") (OtherComp :type "PrimitiveComponent Object Reference") (OtherBodyIndex :type Integer))
  (cast `PlayerCharacter` OtherActor)
  (`PrimitiveComponent.SetMaterial` (`self.Sphere`) 0 "/Game/Assets/Materials/Dome_Red_Mat_Inst.Dome_Red_Mat_Inst")
  (set `self.InSphere` false))

(fn `UserConstructionScript`)