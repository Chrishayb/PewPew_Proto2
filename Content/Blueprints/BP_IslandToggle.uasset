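; BP_IslandToggle is an island actor that swaps its appearance between a real world and an imagined world.
; On BeginPlay it binds handlers to the PortalDefenseGameMode toggle events, printing a message if the cast fails.
; Each handler flips visibility between RealWorldMesh and ImagineWorldMesh so only one shows, without propagating to child components.
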(event `self.ReceiveBeginPlay`
  (bind _asportal_defense_game_mode (cast `PortalDefenseGameMode` (`GameplayStatics.GetGameMode`))
    (:`then`
      (add `PortalDefenseGameMode.OnToggleToImagineWorld` _asportal_defense_game_mode (delegate `OnToImagineWorld`))
      (add `PortalDefenseGameMode.OnToggleToRealWorld` _asportal_defense_game_mode (delegate `OnToRealWorld`)))
    (:`CastFailed`
      (`KismetSystemLibrary.PrintString` "Its currently not "))))

(event `OnToImagineWorld`
  (`self.ToggleToImagineWorld`))

(event `OnToRealWorld`
  (`self.ToggleToRealWorld`))

(fn `ToggleToImagineWorld`
  (`SceneComponent.SetVisibility` (`self.RealWorldMesh`) false false)
  (`SceneComponent.SetVisibility` (`self.ImagineWorldMesh`) true false))

(fn `ToggleToRealWorld`
  (`SceneComponent.SetVisibility` (`self.RealWorldMesh`) true false)
  (`SceneComponent.SetVisibility` (`self.ImagineWorldMesh`) false false))

(fn `UserConstructionScript`)